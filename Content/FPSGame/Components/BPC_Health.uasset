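; BPC_Health is a server-authoritative health component for FPS players, handling damage, healing and reset, with an empty OnRep handler for Health.
; Damage applies only while the game state's round has not ended, and health is clamped between zero and MaxHealth.
; At zero, it casts its owner to BP_FPSPlayerState and reports the death and instigator to BP_FPSGameMode.
; Healing works only on living, injured players and returns whether it applied.
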(fn `CheckDamageRoundEnd`
  (returns (bCanDamage :type Boolean))
  (bind _asbp_fpsgame_state (cast `/Game/FPSGame/Core/BP_FPSGameState` (`GameplayStatics.GetGameState`))
    (:`then`
      (if (not (`/Game/FPSGame/Core/BP_FPSGameState.bRoundEnded` _asbp_fpsgame_state))
        (return true)
        (else
          _)))
    (:`CastFailed`
      _))
  (return false))

(fn `Heal Health`
  (params (HealAmount :type "Float (double-precision)"))
  (returns (bHealed :type Boolean))
  (bind _health (`self.Health`))
  (`/Engine/EditorBlueprintResources/ActorComponentMacros.Switch Has Authority`
    (:`Authority`
      (if (and (> _health 0.0) (< _health (`self.MaxHealth`)) (> HealAmount 0.0))
        (set `self.Health` (`KismetMathLibrary.FClamp` (+ (`self.Health`) HealAmount) 0.0 (`self.MaxHealth`)))
        (return true)
        (else
          _)))
    (:`Remote`
      _))
  (return false))

(fn `OnRep_Health`)

(fn `Receive Damage`
  (params (DamageAmount :type "Float (double-precision)") (`Damage Instigator` :type "Controller Object Reference"))
  (bind _bcandamage (`self.CheckDamageRoundEnd`))
  (if _bcandamage
    (if (and (> DamageAmount 0.0) (`Actor.HasAuthority` (`self.GetOwner`)) (> (`self.Health`) 0.0))
      (set `self.Health` (`KismetMathLibrary.FClamp` (- (`self.Health`) DamageAmount) 0.0 (`self.MaxHealth`)))
      (if (<= (`self.Health`) 0.0)
        (bind _asbp_fpsplayer_state (cast `/Game/FPSGame/Core/BP_FPSPlayerState` (`self.GetOwner`)))
        (bind _asbp_fpsgame_mode (cast `/Game/FPSGame/Blueprint/BP_FPSGameMode` (`GameplayStatics.GetGameMode`)))
        (`/Game/FPSGame/Blueprint/BP_FPSGameMode.HandlePlayerDeath` _asbp_fpsgame_mode _asbp_fpsplayer_state `Damage Instigator`)))))

(fn `ResetHealth`
  (if (`Actor.HasAuthority` (`self.GetOwner`))
    (set `self.Health` (`self.MaxHealth`))))