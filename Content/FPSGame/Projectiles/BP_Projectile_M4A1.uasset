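; M4A1 bullet projectile for the FPS game that damages desktop player characters on impact.
; On a server-authoritative sphere collision hit, it ignores its owner and applies fixed damage through the health component on the victim's PlayerState, passing the instigator controller.
; It destroys itself after hitting a character with the expected PlayerState, or on the server when projectile movement stops.
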(event `self.SphereCollision.OnComponentHit`
  (params (HitComponent :type "PrimitiveComponent Object Reference") (OtherActor :type "Actor Object Reference") (OtherComp :type "PrimitiveComponent Object Reference") (NormalImpulse :type "Vector Structure") (Hit :type "HitResult Structure (by ref)"))
  (`/Engine/EditorBlueprintResources/ActorMacros.Switch Has Authority`
    (:`Authority`
      (if (!= OtherActor (`self.GetOwner`))
        (bind _asbp_desktop_character (cast `/Game/FPSGame/Blueprint/BP_DesktopCharacter` OtherActor))
        (bind _asbp_fpsplayer_state (cast `/Game/FPSGame/Core/BP_FPSPlayerState` (`Pawn.PlayerState` _asbp_desktop_character)))
        (bind _returnvalue (`self.GetComponentByClass` _asbp_fpsplayer_state "/Game/FPSGame/Components/BPC_Health.BPC_Health_C"))
        (`/Engine/EditorBlueprintResources/StandardMacros.IsValid` _returnvalue
          (:`Is Valid`
            (`/Game/FPSGame/Components/BPC_Health.Receive Damage` _returnvalue 20.0 (`self.GetInstigatorController`))
            (`self.K2_DestroyActor`))
          (:`Is Not Valid`
            (`self.K2_DestroyActor`)))))))

(event `self.ProjectileMovement.OnProjectileStop`
  (params (ImpactResult :type "HitResult Structure (by ref)"))
  (`/Engine/EditorBlueprintResources/ActorMacros.Switch Has Authority`
    (:`Authority`
      (`self.K2_DestroyActor`))))

(fn `UserConstructionScript`)