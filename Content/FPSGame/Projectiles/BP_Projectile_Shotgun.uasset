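; Shotgun projectile for the FPS game that damages the desktop characters it hits, with hit logic and destruction run on the server.
; A collision with a non-owner character triggers multicast impact effects on both character and projectile, then applies fixed damage through the health component on the victim's PlayerState.
; It destroys itself after that damage step or when projectile movement stops.
; The effect event picks a Niagara system for character hits, otherwise an explosion emitter.
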(event `self.ProjectileMovement.OnProjectileStop`
  (params (ImpactResult :type "HitResult Structure (by ref)"))
  (`/Engine/EditorBlueprintResources/ActorMacros.Switch Has Authority`
    (:`Authority`
      (`self.K2_DestroyActor`))))

(event `self.SphereCollision.OnComponentHit`
  (params (HitComponent :type "PrimitiveComponent Object Reference") (OtherActor :type "Actor Object Reference") (OtherComp :type "PrimitiveComponent Object Reference") (NormalImpulse :type "Vector Structure") (Hit :type "HitResult Structure (by ref)"))
  (bind (_bblockinghit _binitialoverlap _time _distance _location _impactpoint _normal _impactnormal) (`GameplayStatics.BreakHitResult` Hit))
  (`/Engine/EditorBlueprintResources/ActorMacros.Switch Has Authority`
    (:`Authority`
      (if (!= OtherActor (`self.GetOwner`))
        (bind _asbp_desktop_character (cast `/Game/FPSGame/Blueprint/BP_DesktopCharacter` OtherActor))
        (`/Game/FPSGame/Blueprint/BP_DesktopCharacter.Multicast_PlayImpactFX_Character` _asbp_desktop_character _impactpoint (`KismetMathLibrary.Conv_VectorToRotator` _impactnormal) false)
        (`|ExecutionSequence`
          (:`then_0`
            (`self.Multicast_PlayImpactFX` _impactpoint (`KismetMathLibrary.Conv_VectorToRotator` _impactnormal) true))
          (:`then_1`
            (bind _asbp_fpsplayer_state (cast `/Game/FPSGame/Core/BP_FPSPlayerState` (`Pawn.PlayerState` _asbp_desktop_character)))
            (bind _returnvalue (`self.GetComponentByClass` _asbp_fpsplayer_state "/Game/FPSGame/Components/BPC_Health.BPC_Health_C"))
            (`/Engine/EditorBlueprintResources/StandardMacros.IsValid` _returnvalue
              (:`Is Valid`
                (`/Game/FPSGame/Components/BPC_Health.Receive Damage` _returnvalue 20.0 (`self.GetInstigatorController`))
                (`self.K2_DestroyActor`))
              (:`Is Not Valid`
                (`self.K2_DestroyActor`)))))))))

(event `Multicast_PlayImpactFX`
  (params (ImpactLocation :type "Vector Structure") (ImpactRotation :type "Rotator Structure") (`Is Character Hit` :type Boolean))
  (if `Is Character Hit`
    (bind (_bblockinghit _binitialoverlap _time _distance _location _impactpoint _normal _impactnormal) (`GameplayStatics.BreakHitResult` (stale `self.SphereCollision.OnComponentHit` Hit)))
    (`NiagaraFunctionLibrary.SpawnSystemAtLocation` "/Game/FPSGame/VFX/NS_MuzzleFlash.NS_MuzzleFlash" _impactpoint (`KismetMathLibrary.Conv_VectorToRotator` _impactnormal))
    (else
      (`GameplayStatics.SpawnEmitterAtLocation` "/Game/Model/MilitaryWeapSilver/FX/P_Grenade_Explosion_01.P_Grenade_Explosion_01" ImpactLocation ImpactRotation))))

(fn `UserConstructionScript`)