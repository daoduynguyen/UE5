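; Player state for the FPS game that tracks a player's kills, stores the initial spawn point and triggers respawns.
; AddKill increments Kills, which has an empty RepNotify, and SaveInitialSpawn records the spawn transform only the first time it is called.
; ScheduleRespawn waits a short delay, then asks BP_FPSGameMode to respawn this player.
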(event `Schedule Respawn`
  (`KismetSystemLibrary.Delay` 2.0)
  (bind _asbp_fpsgame_mode (cast `/Game/FPSGame/Blueprint/BP_FPSGameMode` (`GameplayStatics.GetGameMode`)))
  (`/Game/FPSGame/Blueprint/BP_FPSGameMode.Respawn Single Player` _asbp_fpsgame_mode self))

(fn `AddKill`
  (returns (NewKills :type Integer))
  (bind _output_get (set `self.Kills` (+ (`self.Kills`) 1)))
  (return _output_get))

(fn `OnRep_Kills`)

(fn `SaveInitialSpawn`
  (params (SpawnTransform :type "Transform Structure"))
  (if (not (`self.bSpawnSaved`))
    (set `self.InitialSpawnTransform` SpawnTransform)
    (set `self.bSpawnSaved` true)))

(fn `UserConstructionScript`)