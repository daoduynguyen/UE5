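; Player controller for the FPS game that manages the local HUD, round result screen and kill feed.
; On BeginPlay the local controller adds crosshair and health bar widgets, and client events forward kill messages to the health bar.
; Showing a round result locks movement and look for UI input, while resetting restores game control.
; Restart requests reach the game mode's RestartCombatRound only for a locally controlled controller.
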(event `self.ReceiveBeginPlay`
  (if (`self.IsLocalController`)
    (bind _returnvalue (`|CreateWidget` "/Game/FPSGame/UI/BP_Crosshair.BP_Crosshair_C" self))
    (`UserWidget.AddToViewport` _returnvalue 0)
    (bind _returnvalue_2 (`|CreateWidget` "/Game/FPSGame/UI/BP_HealthBar.BP_HealthBar_C" self))
    (`UserWidget.AddToViewport` _returnvalue_2 0)))

(event `Client_ShowRoundResult`
  (params (bWon :type Boolean))
  (`self.SetIgnoreMoveInput` true)
  (`self.SetIgnoreLookInput` true)
  (bind _returnvalue (`|CreateWidget` "/Game/FPSGame/UI/BP_RoundResult.BP_RoundResult_C" self bWon))
  (set `self.RoundResultWidget` _returnvalue)
  (`UserWidget.AddToViewport` _returnvalue 0)
  (set `self.bShowMouseCursor` true)
  (`WidgetBlueprintLibrary.SetInputMode_GameAndUIEx` self _returnvalue))

(event `Client_ResetRoundUi`
  (bind _roundresultwidget (`self.RoundResultWidget`))
  (`/Engine/EditorBlueprintResources/StandardMacros.IsValid` _roundresultwidget
    (:`Is Valid`
      (`Widget.RemoveFromParent` _roundresultwidget)
      (`self.UpdateControl`))
    (:`Is Not Valid`
      (`self.UpdateControl`))))

(event `Server_RequestRestart`
  (if (`self.IsLocalController`)
    (bind _asbp_fpsgame_mode (cast `/Game/FPSGame/Blueprint/BP_FPSGameMode` (`GameplayStatics.GetGameMode`)))
    (`/Game/FPSGame/Blueprint/BP_FPSGameMode.RestartCombatRound` _asbp_fpsgame_mode)))

(event `Client_ShowKillFeed`
  (params (KillerName :type String) (VictimName :type String))
  (bind _foundwidgets (`WidgetBlueprintLibrary.GetAllWidgetsOfClass` "/Game/FPSGame/UI/BP_HealthBar.BP_HealthBar_C"))
  (`/Game/FPSGame/UI/BP_HealthBar.ShowKillFeed` (`|GetArrayItem` _foundwidgets) KillerName VictimName))

(fn `UpdateControl`
  (`self.SetIgnoreMoveInput` false)
  (`self.SetIgnoreLookInput` false)
  (set `self.bShowMouseCursor` false)
  (`WidgetBlueprintLibrary.SetInputMode_GameOnly` self))

(fn `UserConstructionScript`)