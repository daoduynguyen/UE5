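; BP_WeaponPickup is a floating, spinning weapon pickup that swaps its gun and ammo with an overlapping BP_DesktopCharacter.
; Server-only overlap calls TryPickupWeapon, which destroys the pickup if the character's old weapon type is zero, otherwise stores that weapon and ammo.
; CanPickup blocks repeat swaps until a character ends overlap.
; WeaponType selects the M4A1 or shotgun mesh on construction, BeginPlay, swap and RepNotify.
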(event `self.ReceiveBeginPlay`
  (`self.UpdatePickupMesh`))

(event `self.PickupSphere.OnComponentBeginOverlap`
  (params (OverlappedComponent :type "PrimitiveComponent Object Reference") (OtherActor :type "Actor Object Reference") (OtherComp :type "PrimitiveComponent Object Reference") (OtherBodyIndex :type Integer) (bFromSweep :type Boolean) (SweepResult :type "HitResult Structure (by ref)"))
  (`/Engine/EditorBlueprintResources/ActorMacros.Switch Has Authority`
    (:`Authority`
      (bind _asbp_desktop_character (cast `/Game/FPSGame/Blueprint/BP_DesktopCharacter` OtherActor))
      (`self.TryPickupWeapon` _asbp_desktop_character))))

(event `self.PickupSphere.OnComponentEndOverlap`
  (params (OverlappedComponent :type "PrimitiveComponent Object Reference") (OtherActor :type "Actor Object Reference") (OtherComp :type "PrimitiveComponent Object Reference") (OtherBodyIndex :type Integer))
  (`/Engine/EditorBlueprintResources/ActorMacros.Switch Has Authority`
    (:`Authority`
      (cast `/Game/FPSGame/Blueprint/BP_DesktopCharacter` OtherActor)
      (set `self.bCanPickup` true))))

(event `self.ReceiveTick`
  (params (DeltaSeconds :type "Float (single-precision)"))
  (`SceneComponent.K2_SetRelativeLocation` (`self.PickupMesh`) (+ (* (`KismetMathLibrary.Sin` (* (`self.FloatSpeed`) (`KismetSystemLibrary.GetGameTimeInSeconds`))) (`self.FloatHeight`)) (`self.StartLocation`)) false false)
  (`SceneComponent.K2_AddLocalRotation` (`self.PickupMesh`) (`KismetMathLibrary.MakeRotator` 0.0 0.0 (* DeltaSeconds 45.0)) false false))

(fn `OnRep_MagazineAmmo`)

(fn `OnRep_WeaponType`
  (`self.UpdatePickupMesh`))

(fn `TryPickupWeapon`
  (params (PickingCharacter :type "/Game/FPSGame/Blueprint/BP_DesktopCharacter Object Reference"))
  (locals (OldAmmo :type Integer) (OldMagazineAmmo :type Integer))
  (bind _bp_weapon_component (`/Game/FPSGame/Blueprint/BP_DesktopCharacter.BP_Weapon_Component` PickingCharacter))
  (if (`self.bCanPickup`)
    (set `self.bCanPickup` false)
    (set `self.OldWeaponType` (`/Game/FPSGame/Blueprint/BP_DesktopCharacter.EquippedWeaponType` PickingCharacter))
    (set `local.OldAmmo` (`/Game/FPSGame/Components/BP_Weapon_Component.CurrentAmmo` _bp_weapon_component))
    (set `local.OldMagazineAmmo` (`/Game/FPSGame/Components/BP_Weapon_Component.MagazineAmmo` _bp_weapon_component))
    (set `/Game/FPSGame/Blueprint/BP_DesktopCharacter.EquippedWeaponType` (`self.WeaponType`) PickingCharacter)
    (set `/Game/FPSGame/Components/BP_Weapon_Component.CurrentAmmo` (`self.Ammo`) _bp_weapon_component)
    (set `/Game/FPSGame/Components/BP_Weapon_Component.MagazineAmmo` (`self.MagazineAmmo`) _bp_weapon_component)
    (`/Game/FPSGame/Blueprint/BP_DesktopCharacter.UpdateEquippedWeaponMesh` PickingCharacter)
    (if (== (`self.OldWeaponType`) 0)
      (`self.K2_DestroyActor`)
      (else
        (set `self.WeaponType` (`self.OldWeaponType`))
        (set `self.Ammo` (`local.OldAmmo`))
        (set `self.MagazineAmmo` (`local.OldMagazineAmmo`))
        (`self.UpdatePickupMesh`)))))

(fn `UpdatePickupMesh`
  (bind _pickupmesh (`self.PickupMesh`))
  (switch `/Game/FPSGame/Blueprint/E_WeaponType` (`self.WeaponType`)
    (:`NewEnumerator0`
      (`StaticMeshComponent.SetStaticMesh` _pickupmesh "/Game/FPSGame/Environment/Weapon_01/gun_m4a1.gun_m4a1"))
    (:`NewEnumerator1`
      (`StaticMeshComponent.SetStaticMesh` _pickupmesh "/Game/FPSGame/Environment/Weapon_03/remington_870_shotgun.remington_870_shotgun"))))

(fn `UserConstructionScript`
  (`self.UpdatePickupMesh`))