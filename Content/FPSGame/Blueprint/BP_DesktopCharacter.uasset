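; Desktop first-person player character for a multiplayer shooter, handling Enhanced Input movement, look, jump, shooting and reload.
; Fire and reload go through server events to BPWeaponComponent, with a looping timer repeating shots while fire is held.
; Replicated EquippedWeaponType updates first-person and world weapon meshes and selects the multicast muzzle flash.
; A retry timer binds the overhead health widget to the PlayerState's HealthComponent; Tick yaws it toward the local camera.
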(event `self.ReceiveBeginPlay`
  (bind _returnvalue (`self.GetController`))
  (`|ExecutionSequence`
    (:`then_0`
      (`/Engine/EditorBlueprintResources/StandardMacros.IsValid` _returnvalue
        (:`Is Valid`
          (if (`Controller.IsLocalController` _returnvalue)
            (bind _asplayer_controller (cast `PlayerController` _returnvalue))
            (bind _returnvalue_2 (pcsubsystem `EnhancedInputLocalPlayerSubsystem` _asplayer_controller))
            (`EnhancedInputSubsystemInterface.AddMappingContext` _returnvalue_2 "/Game/FirstPerson/Input/IMC_Default.IMC_Default" 0 (struct))
            (`EnhancedInputSubsystemInterface.AddMappingContext` _returnvalue_2 "/Game/FirstPerson/Input/IMC_Weapons.IMC_Weapons" 1 (struct))))))
    (:`then_1`
      (bind _returnvalue_3 (`KismetSystemLibrary.K2_SetTimerDelegate` (delegate `TryInitHealth`) 0.1 true)))
    (:`then_2`
      (`self.UpdateEquippedWeaponMesh`))))

(event `TryInitHealth`
  (bind _asbp_head_health (cast `/Game/FPSGame/UI/BP_HeadHealth` (`WidgetComponent.GetUserWidgetObject` (`self.WC_HeadHealth`))))
  (bind _asbp_fpsplayer_state (cast `/Game/FPSGame/Core/BP_FPSPlayerState` (`self.PlayerState`)))
  (set `/Game/FPSGame/UI/BP_HeadHealth.HealthComponent` (`/Game/FPSGame/Core/BP_FPSPlayerState.HealthComponent` _asbp_fpsplayer_state) _asbp_head_health)
  (`KismetSystemLibrary.K2_ClearAndInvalidateTimerHandle` (stale `self.ReceiveBeginPlay` _returnvalue_3)))

(event `EnhancedInput|/Game/FirstPerson/Input/Actions/IA_Move`
  (params (ActionValue :type "Vector2D Structure") (ElapsedSeconds :type "Float (double-precision)") (TriggeredSeconds :type "Float (double-precision)") (InputAction :type "InputAction Object Reference" :default "/Game/FirstPerson/Input/Actions/IA_Move.IA_Move"))
  (bind _returnvalue (`KismetMathLibrary.MakeRotator` 0.0 0.0 (.yaw (`self.GetControlRotation`))))
  (:`Triggered`
    (`self.AddMovementInput` (`KismetMathLibrary.GetForwardVector` _returnvalue) ActionValue_Y)
    (`self.AddMovementInput` (`KismetMathLibrary.GetRightVector` _returnvalue) ActionValue_X)))

(event `EnhancedInput|/Game/FirstPerson/Input/Actions/IA_Look`
  (params (ActionValue :type "Vector2D Structure") (ElapsedSeconds :type "Float (double-precision)") (TriggeredSeconds :type "Float (double-precision)") (InputAction :type "InputAction Object Reference" :default "/Game/FirstPerson/Input/Actions/IA_Look.IA_Look"))
  (:`Triggered`
    (`self.AddControllerYawInput` ActionValue_X)
    (`self.AddControllerPitchInput` ActionValue_Y)))

(event `EnhancedInput|/Game/FirstPerson/Input/Actions/IA_Jump`
  (params (ActionValue :type Boolean) (ElapsedSeconds :type "Float (double-precision)") (TriggeredSeconds :type "Float (double-precision)") (InputAction :type "InputAction Object Reference" :default "/Game/FirstPerson/Input/Actions/IA_Jump.IA_Jump"))
  (:`Triggered`
    (`self.Jump`))
  (:`Completed`
    (`self.StopJumping`)))

(event `EnhancedInput|/Game/FirstPerson/Input/Actions/IA_Reload`
  (params (ActionValue :type Boolean) (ElapsedSeconds :type "Float (double-precision)") (TriggeredSeconds :type "Float (double-precision)") (InputAction :type "InputAction Object Reference" :default "/Game/FirstPerson/Input/Actions/IA_Reload.IA_Reload"))
  (:`Started`
    (`self.Server_Reload`)))

(event `EnhancedInput|/Game/FirstPerson/Input/Actions/IA_Shoot`
  (params (ActionValue :type Boolean) (ElapsedSeconds :type "Float (double-precision)") (TriggeredSeconds :type "Float (double-precision)") (InputAction :type "InputAction Object Reference" :default "/Game/FirstPerson/Input/Actions/IA_Shoot.IA_Shoot"))
  (:`Started`
    (`self.Server_StartFire`))
  (:`Canceled`
    (`self.Server_StopFire`))
  (:`Completed`
    (`self.Server_StopFire`)))

(event `Server_Fire`
  (params (Rotation :type "Rotator Structure"))
  (`/Game/FPSGame/Components/BP_Weapon_Component.Fire` (`self.BP_Weapon_Component`) Rotation))

(event `self.ReceiveTick`
  (params (DeltaSeconds :type "Float (single-precision)"))
  (bind _wc_headhealth (`self.WC_HeadHealth`))
  (`SceneComponent.K2_SetWorldRotation` _wc_headhealth (`KismetMathLibrary.MakeRotator` 0.0 0.0 (.yaw (`KismetMathLibrary.FindLookAtRotation` (`SceneComponent.K2_GetComponentLocation` _wc_headhealth) (`PlayerCameraManager.GetCameraLocation` (`GameplayStatics.GetPlayerCameraManager` 0))))) false false))

(event `Multicast_PlayMuzzleFlash`
  (switch `/Game/FPSGame/Blueprint/E_WeaponType` (`self.EquippedWeaponType`)
    (:`NewEnumerator0`
      (`GameplayStatics.SpawnEmitterAttached` "/Game/Model/MilitaryWeapSilver/FX/P_AssaultRifle_MuzzleFlash.P_AssaultRifle_MuzzleFlash" (`self.MuzzlePoint`)))
    (:`NewEnumerator1`
      (`GameplayStatics.SpawnEmitterAttached` "/Game/Model/MilitaryWeapSilver/FX/P_Shotgun_MuzzleFlash_01.P_Shotgun_MuzzleFlash_01" (`self.MuzzlePoint`)))))

(event `FireOnce`
  (if (`self.bIsHoldingFire`)
    (`self.Server_Fire` (`self.GetBaseAimRotation`))))

(event `Server_StartFire`
  (set `self.bIsHoldingFire` true)
  (if (not (`KismetSystemLibrary.K2_IsTimerActiveHandle` (`self.FireTimerHandle`)))
    (`|ExecutionSequence`
      (:`then_0`
        (bind _returnvalue (`KismetSystemLibrary.K2_SetTimerDelegate` (delegate `FireOnce`) (`self.FireInterval`) true))
        (set `self.FireTimerHandle` _returnvalue))
      (:`then_1`
        (`self.FireOnce`)))))

(event `Server_StopFire`
  (set `self.bIsHoldingFire` false)
  (`KismetSystemLibrary.K2_ClearAndInvalidateTimerHandle` (`self.FireTimerHandle`)))

(event `Server_Reload`
  (`/Game/FPSGame/Components/BP_Weapon_Component.AutoReload` (`self.BP_Weapon_Component`)))

(fn `CalculateAimRotation`
  (returns (AimRotation :type "Rotator Structure"))
  (bind _aimtargetpoint (`self.CalculateAimTargetPoint`))
  (return (`KismetMathLibrary.FindLookAtRotation` (`SceneComponent.K2_GetComponentLocation` (`self.FP_MuzzlePoint`)) _aimtargetpoint)))

(fn `CalculateAimTargetPoint`
  (returns (AimTargetPoint :type "Vector Structure"))
  (bind _camera_fp (`self.Camera_FP`))
  (return (+ (`SceneComponent.K2_GetComponentLocation` _camera_fp) (* (`SceneComponent.GetForwardVector` _camera_fp) (`KismetMathLibrary.Conv_DoubleToVector` 100000.0)))))

(fn `OnRep_EquippedWeaponType`
  (`self.UpdateEquippedWeaponMesh`))

(fn `UpdateEquippedWeaponMesh`
  (switch `/Game/FPSGame/Blueprint/E_WeaponType` (`self.EquippedWeaponType`)
    (:`NewEnumerator2`
      (`StaticMeshComponent.SetStaticMesh` (`self.EquippedWeaponMesh`) null)
      (`StaticMeshComponent.SetStaticMesh` (`self.FP_EquippedWeaponMesh`) null))
    (:`NewEnumerator0`
      (`StaticMeshComponent.SetStaticMesh` (`self.EquippedWeaponMesh`) "/Game/FPSGame/Environment/Weapon_01/gun_m4a1.gun_m4a1")
      (`StaticMeshComponent.SetStaticMesh` (`self.FP_EquippedWeaponMesh`) "/Game/FPSGame/Environment/Weapon_01/gun_m4a1.gun_m4a1"))
    (:`NewEnumerator1`
      (`StaticMeshComponent.SetStaticMesh` (`self.EquippedWeaponMesh`) "/Game/FPSGame/Environment/Weapon_03/remington_870_shotgun.remington_870_shotgun")
      (`StaticMeshComponent.SetStaticMesh` (`self.FP_EquippedWeaponMesh`) "/Game/FPSGame/Environment/Weapon_03/remington_870_shotgun.remington_870_shotgun"))))

(fn `UserConstructionScript`)