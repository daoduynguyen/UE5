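; BP_HealthPickUp is a health pickup that bobs in place and heals a player who touches it.
; Tick offsets the HealHealth component's relative location with a sine of game time, scaled by float speed and height.
; On sphere overlap, only the authority casts to BP_DesktopCharacter, calls HealHealth on the HealthComponent in its BP_FPSPlayerState, and destroys the pickup only if that call succeeds.
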(event `self.ReceiveBeginPlay`
  (set `self.StartLocation` (`SceneComponent.RelativeLocation` (`self.HealHealth`))))

(event `self.ReceiveTick`
  (params (DeltaSeconds :type "Float (single-precision)"))
  (`SceneComponent.K2_SetRelativeLocation` (`self.HealHealth`) (+ (* (`KismetMathLibrary.Sin` (* (`self.FloatSpeed`) (`KismetSystemLibrary.GetGameTimeInSeconds`))) (`self.FloatHeight`)) (`self.StartLocation`)) false false))

(event `self.PickupSphere.OnComponentBeginOverlap`
  (params (OverlappedComponent :type "PrimitiveComponent Object Reference") (OtherActor :type "Actor Object Reference") (OtherComp :type "PrimitiveComponent Object Reference") (OtherBodyIndex :type Integer) (bFromSweep :type Boolean) (SweepResult :type "HitResult Structure (by ref)"))
  (`/Engine/EditorBlueprintResources/ActorMacros.Switch Has Authority`
    (:`Authority`
      (bind _asbp_desktop_character (cast `/Game/FPSGame/Blueprint/BP_DesktopCharacter` OtherActor))
      (bind _asbp_fpsplayer_state (cast `/Game/FPSGame/Core/BP_FPSPlayerState` (`Pawn.PlayerState` _asbp_desktop_character)))
      (bind _healthcomponent (`/Game/FPSGame/Core/BP_FPSPlayerState.HealthComponent` _asbp_fpsplayer_state))
      (`/Engine/EditorBlueprintResources/StandardMacros.IsValid` _healthcomponent
        (:`Is Valid`
          (bind _bhealed (`/Game/FPSGame/Components/BPC_Health.Heal Health` _healthcomponent 30.0))
          (if _bhealed
            (`self.K2_DestroyActor`)))))))

(fn `UserConstructionScript`)