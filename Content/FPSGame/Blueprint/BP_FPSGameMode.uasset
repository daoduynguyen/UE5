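; Game mode for a kill-target FPS match that names joining players Player1 or Player2 and runs deaths, respawns and round restarts.
; Guarded death handling destroys the pawn, credits the killer and broadcasts the kill feed.
; It then either schedules a respawn at the saved spawn transform or, at KillsToWin, ends the round with per-client results.
; Restarting clears GameState and PlayerState match data, resets health, respawns everyone and resets client UI.
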(event `self.K2_PostLogin`
  (params (NewPlayer :type "PlayerController Object Reference"))
  (bind _returnvalue (`self.GetNumPlayers` self))
  (if (== _returnvalue 1)
    (`self.ChangeName` self NewPlayer "Player1" true)
    (else
      (`self.ChangeName` self NewPlayer "Player2" true))))

(event `self.ReceiveBeginPlay`
  (bind _asbp_fpsgame_state (cast `/Game/FPSGame/Core/BP_FPSGameState` (`GameplayStatics.GetGameState`)))
  (set `self.GameStateRef` _asbp_fpsgame_state))

(event `EndCombatRound`
  (params (LoserPlayerState :type "/Game/FPSGame/Core/BP_FPSPlayerState Object Reference"))
  (bind _asbp_fpsgame_state (cast `/Game/FPSGame/Core/BP_FPSGameState` (`GameplayStatics.GetGameState`)))
  (if (not (`/Game/FPSGame/Core/BP_FPSGameState.bRoundEnded` _asbp_fpsgame_state))
    (set `/Game/FPSGame/Core/BP_FPSGameState.bRoundEnded` true _asbp_fpsgame_state)
    (bind _outactors (`GameplayStatics.GetAllActorsOfClass` "/Game/FPSGame/Core/BP_FPSPlayerController.BP_FPSPlayerController_C"))
    (for _array_element _outactors
      (`/Game/FPSGame/Core/BP_FPSPlayerController.Client_ShowRoundResult` _array_element (!= (`Controller.PlayerState` _array_element) LoserPlayerState)))))

(event `RestartCombatRound`
  (bind _asbp_fpsgame_state (cast `/Game/FPSGame/Core/BP_FPSGameState` (`GameplayStatics.GetGameState`)))
  (if (`/Game/FPSGame/Core/BP_FPSGameState.bRoundEnded` _asbp_fpsgame_state)
    (set `/Game/FPSGame/Core/BP_FPSGameState.bMatchEnded` false _asbp_fpsgame_state)
    (set `/Game/FPSGame/Core/BP_FPSGameState.WinnerPlayerState` null _asbp_fpsgame_state)
    (bind _outactors (`GameplayStatics.GetAllActorsOfClass` "/Game/FPSGame/Core/BP_FPSPlayerController.BP_FPSPlayerController_C"))
    (for _array_element _outactors
      (bind _asbp_fpsplayer_state (cast `/Game/FPSGame/Core/BP_FPSPlayerState` (`Controller.PlayerState` _array_element)))
      (set `/Game/FPSGame/Core/BP_FPSPlayerState.bWaitingRespawn` false _asbp_fpsplayer_state)
      (set `/Game/FPSGame/Core/BP_FPSPlayerState.Kills` 0 _asbp_fpsplayer_state)
      (bind _healthcomponent (`/Game/FPSGame/Core/BP_FPSPlayerState.HealthComponent` _asbp_fpsplayer_state))
      (`/Engine/EditorBlueprintResources/StandardMacros.IsValid` _healthcomponent
        (:`Is Valid`
          (`/Game/FPSGame/Components/BPC_Health.ResetHealth` _healthcomponent))))
    (for _array_element_2 _outactors
      (bind _returnvalue (`Controller.K2_GetPawn` _array_element_2))
      (`/Engine/EditorBlueprintResources/StandardMacros.IsValid` _returnvalue
        (:`Is Valid`
          (`self.K2_DestroyActor` _returnvalue)
          (`self.RestartPlayer` _array_element_2))
        (:`Is Not Valid`
          (`self.RestartPlayer` _array_element_2))))
    (set `/Game/FPSGame/Core/BP_FPSGameState.bRoundEnded` false _asbp_fpsgame_state)
    (bind _outactors_2 (`GameplayStatics.GetAllActorsOfClass` "/Game/FPSGame/Core/BP_FPSPlayerController.BP_FPSPlayerController_C"))
    (for _array_element_3 _outactors_2
      (`/Game/FPSGame/Core/BP_FPSPlayerController.Client_ResetRoundUi` _array_element_3))))

(event `HandlePlayerDeath`
  (params (LoserPlayerState :type "/Game/FPSGame/Core/BP_FPSPlayerState Object Reference") (`Damage Instigator` :type "Controller Object Reference"))
  (bind _returnvalue (`PlayerState.GetPawn` LoserPlayerState))
  (bind _bcanhandle (`self.Can Handle Death` LoserPlayerState))
  (if _bcanhandle
    (set `/Game/FPSGame/Core/BP_FPSPlayerState.bWaitingRespawn` true LoserPlayerState)
    (`|ExecutionSequence`
      (:`then_0`
        (`/Engine/EditorBlueprintResources/StandardMacros.IsValid` _returnvalue
          (:`Is Valid`
            (`self.K2_DestroyActor` _returnvalue))))
      (:`then_1`
        (`/Engine/EditorBlueprintResources/StandardMacros.IsValid` `Damage Instigator`
          (:`Is Valid`
            (bind _asbp_fpsplayer_state (cast `/Game/FPSGame/Core/BP_FPSPlayerState` (`Controller.PlayerState` `Damage Instigator`)))
            (if (!= _asbp_fpsplayer_state LoserPlayerState)
              (bind _newkills (`/Game/FPSGame/Core/BP_FPSPlayerState.AddKill` _asbp_fpsplayer_state))
              (`self.BroadCastKillFeed` _asbp_fpsplayer_state LoserPlayerState)
              (if (>= _newkills (`/Game/FPSGame/Core/BP_FPSGameState.KillsToWin` (`self.GameStateRef`)))
                (set `/Game/FPSGame/Core/BP_FPSGameState.WinnerPlayerState` _asbp_fpsplayer_state (`self.GameStateRef`))
                (set `/Game/FPSGame/Core/BP_FPSGameState.bMatchEnded` true (`self.GameStateRef`))
                (`self.EndCombatRound` LoserPlayerState)
                (else
                  (`/Game/FPSGame/Core/BP_FPSPlayerState.Schedule Respawn` LoserPlayerState))))))))))

(event `Respawn Single Player`
  (params (LoserPlayerState :type "/Game/FPSGame/Core/BP_FPSPlayerState Object Reference"))
  (bind _returnvalue (`PlayerState.GetPlayerController` LoserPlayerState))
  (bind _btryrespawn (`self.Try Respawn Player` LoserPlayerState))
  (if _btryrespawn
    (`/Game/FPSGame/Components/BPC_Health.ResetHealth` (`/Game/FPSGame/Core/BP_FPSPlayerState.HealthComponent` LoserPlayerState))
    (`self.RestartPlayerAtTransform` _returnvalue (`/Game/FPSGame/Core/BP_FPSPlayerState.InitialSpawnTransform` LoserPlayerState))
    (`/Engine/EditorBlueprintResources/StandardMacros.IsValid` (`Controller.K2_GetPawn` _returnvalue)
      (:`Is Valid`
        (set `/Game/FPSGame/Core/BP_FPSPlayerState.bWaitingRespawn` false LoserPlayerState))
      (:`Is Not Valid`
        (`KismetSystemLibrary.PrintString` "Failed")))))

(fn `BroadCastKillFeed`
  (params (KillerPS :type "/Game/FPSGame/Core/BP_FPSPlayerState Object Reference") (LoserPS :type "/Game/FPSGame/Core/BP_FPSPlayerState Object Reference"))
  (bind _outactors (`GameplayStatics.GetAllActorsOfClass` "/Game/FPSGame/Core/BP_FPSPlayerController.BP_FPSPlayerController_C"))
  (for _array_element _outactors
    (`/Game/FPSGame/Core/BP_FPSPlayerController.Client_ShowKillFeed` _array_element (`PlayerState.GetPlayerName` KillerPS) (`PlayerState.GetPlayerName` LoserPS))))

(fn `Can Handle Death`
  (params (LoserPS :type "/Game/FPSGame/Core/BP_FPSPlayerState Object Reference"))
  (returns (bCanHandle :type Boolean))
  (bind _gamestateref (`self.GameStateRef`))
  (`/Engine/EditorBlueprintResources/StandardMacros.IsValid` LoserPS
    (:`Is Valid`
      (`/Engine/EditorBlueprintResources/StandardMacros.IsValid` _gamestateref
        (:`Is Valid`
          (if (not (`/Game/FPSGame/Core/BP_FPSGameState.bMatchEnded` _gamestateref))
            (if (not (`/Game/FPSGame/Core/BP_FPSPlayerState.bWaitingRespawn` LoserPS))
              (return true)
              (else
                (return false)))))))))

(fn `Try Respawn Player`
  (params (LoserPS :type "/Game/FPSGame/Core/BP_FPSPlayerState Object Reference"))
  (returns (bTryRespawn :type Boolean))
  (bind _returnvalue (`PlayerState.GetPlayerController` LoserPS))
  (`/Engine/EditorBlueprintResources/StandardMacros.IsValid` LoserPS
    (:`Is Valid`
      (`/Engine/EditorBlueprintResources/StandardMacros.IsValid` (`self.GameStateRef`)
        (:`Is Valid`
          (if (not (`/Game/FPSGame/Core/BP_FPSGameState.bMatchEnded` (`self.GameStateRef`)))
            (if (`/Game/FPSGame/Core/BP_FPSPlayerState.bWaitingRespawn` LoserPS)
              (if (`/Game/FPSGame/Core/BP_FPSPlayerState.bSpawnSaved` LoserPS)
                (`/Engine/EditorBlueprintResources/StandardMacros.IsValid` _returnvalue
                  (:`Is Valid`
                    (`/Engine/EditorBlueprintResources/StandardMacros.IsValid` (`Controller.K2_GetPawn` _returnvalue)
                      (:`Is Not Valid`
                        (`/Engine/EditorBlueprintResources/StandardMacros.IsValid` (`/Game/FPSGame/Core/BP_FPSPlayerState.HealthComponent` LoserPS)
                          (:`Is Valid`
                            (return true))
                          (:`Is Not Valid`
                            (return false)))))))))))))))

(fn `UserConstructionScript`)